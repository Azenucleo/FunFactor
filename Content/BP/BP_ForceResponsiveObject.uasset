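; Actor that stays static until a force event launches its StaticMesh as a physics object.
; ApplyForce pushes the mesh away from an origin, ApplyForcewithDirection along a given vector; both enable simulation and apply a mass-independent impulse scaled by Power.
; ResetForce stops simulation, moves the actor to the mesh's current location and reattaches the mesh to the root, keeping its world transform.
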(event `/Game/BP/BPI_Force.ApplyForce`
  (params (`force origin` :type "Vector Structure") (power :type "Float (double-precision)"))
  (bind _staticmesh (`self.StaticMesh`))
  (`PrimitiveComponent.SetSimulatePhysics` _staticmesh true)
  (`PrimitiveComponent.AddImpulse` _staticmesh (* (`KismetMathLibrary.Normal` (- (`SceneComponent.K2_GetComponentLocation` (`self.StaticMesh`)) `force origin`)) power) "None" true))

(event `/Game/BP/BPI_Force.ApplyForceWithDirection`
  (params (`Direction vector` :type "Vector Structure") (power :type "Float (double-precision)"))
  (bind _staticmesh (`self.StaticMesh`))
  (`PrimitiveComponent.SetSimulatePhysics` _staticmesh true)
  (`PrimitiveComponent.AddImpulse` _staticmesh (* `Direction vector` power) "None" true))

(event `/Game/BP/BPI_Force.ResetForce`
  (bind _staticmesh (`self.StaticMesh`))
  (if (`SceneComponent.IsSimulatingPhysics` _staticmesh "None")
    (`PrimitiveComponent.SetSimulatePhysics` _staticmesh false)
    (`self.K2_SetActorLocation` (`SceneComponent.K2_GetComponentLocation` _staticmesh))
    (`SceneComponent.K2_AttachToComponent` (`self.StaticMesh`) (`self.DefaultSceneRoot`) "None" "KeepWorld" "KeepWorld" "KeepWorld" true)))

(fn `UserConstructionScript`)